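; Game jam GameMode that starts the music and restores saved audio settings on BeginPlay.
; It loads the SG_Audio save slot, or creates a new save object if none exists.
; The saved Master, Music and SFX volumes are applied as sound class overrides on SCM_Default, pushing the mix each time.
; The save is written back to the slot after each of the three overrides.
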(event EventBeginPlay
  ;[1 1 1] Setup Audio
  (Audio|SpawnSound2D "/Game/Audio/Music/MS_Music.MS_Music" 1.0 1.0 0.0 0)
  (bind _returnvalue (SaveGame|DoesSaveGameExist "SG_Audio"))
  (if _returnvalue
    (bind _returnvalue_2 (SaveGame|LoadGamefromSlot "SG_Audio"))
    (bind _assg_audio (Utilities|Casting|CastToSG_Audio _returnvalue_2))
    (Variables|Default|SetSaveGameAudioRef _assg_audio)
    (else
      (bind _returnvalue_3 (SaveGame|CreateSaveGameObject "/Game/Audio/Sounds/Settings/SG_Audio.SG_Audio_C"))
      (Variables|Default|SetSaveGameAudioRef _returnvalue_3)))
  (Utilities|FlowControl|Sequence
    (:then_0
      (Audio|SetSoundMixClassOverride "/Game/Audio/Sounds/Settings/SCM_Default.SCM_Default" "/Game/Audio/Sounds/Settings/SC_Master.SC_Master" (Variables|/Game/Audio/Sounds/Settings/SG_Audio.SG_Audio_C|GetMasterValue (Variables|Default|GetSaveGameAudioRef)) 1.0 0.0 true)
      (Audio|PushSoundMixModifier "/Game/Audio/Sounds/Settings/SCM_Default.SCM_Default"))
    (:then_1
      (Audio|SetSoundMixClassOverride "/Game/Audio/Sounds/Settings/SCM_Default.SCM_Default" "/Game/Audio/Sounds/Settings/SC_Music.SC_Music" (Variables|/Game/Audio/Sounds/Settings/SG_Audio.SG_Audio_C|GetMusicValue (Variables|Default|GetSaveGameAudioRef)) 1.0 0.0 true)
      (Audio|PushSoundMixModifier "/Game/Audio/Sounds/Settings/SCM_Default.SCM_Default"))
    (:then_2
      (Audio|SetSoundMixClassOverride "/Game/Audio/Sounds/Settings/SCM_Default.SCM_Default" "/Game/Audio/Sounds/Settings/SC_Sounds.SC_Sounds" (Variables|/Game/Audio/Sounds/Settings/SG_Audio.SG_Audio_C|GetSFXValue (Variables|Default|GetSaveGameAudioRef)) 1.0 0.0 true)
      (Audio|PushSoundMixModifier "/Game/Audio/Sounds/Settings/SCM_Default.SCM_Default")))
  (SaveGame|SaveGametoSlot (Variables|Default|GetSaveGameAudioRef) "SG_Audio"))

(fn ConstructionScript)