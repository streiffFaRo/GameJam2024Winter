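; Coin pickup that the player collects by overlapping it.
; It registers with the game mode on BeginPlay through an interface-style message.
; On first overlap with a Player-tagged actor it plays a sound, hides its mesh, disables collision, flags itself collected and notifies the game mode.
; The other counter and registration functions are empty stubs, and the count-widget-and-pause logic is unconnected.
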(event OnComponentBeginOverlap(Collision)
  (params (OverlappedComponent :type Primitive%20Component%20Object%20Reference) (OtherActor :type Actor%20Object%20Reference) (OtherComp :type Primitive%20Component%20Object%20Reference) (OtherBodyIndex :type Integer) (bFromSweep :type Boolean) (SweepResult :type Hit%20Result%20Structure%20%28by%20ref%29))
  (if (Actor|ActorHasTag OtherActor "Player")
    (if (not (Variables|Data|GetbCollected))
      (Audio|PlaySound2D "/Engine/VREditor/Sounds/UI/Click_on_Button.Click_on_Button" 1.0 1.0 0.0 0 0)
      (CallFunction|IsCollected))))

(event EventBeginPlay
  ;[0.4773 1 0.4503] Begin
  (Class|BPICollectable|RegisterNewCollectable(Message) (Game|GetGameMode) self))

(fn ConstructionScript)

(fn CollectableCounter
  (return))

(fn GetNumCollectables
  (return 0))

(fn IsCollected
  (params (CollectableRef :type Actor%20Object%20Reference))
  (Utilities|FlowControl|Sequence
    (:then_0
      (Development|SetHiddeninGame (Variables|Default|GetCollectableMesh) true false)
      (Collision|SetCollisionEnabled (Variables|Default|GetCollision) "NoCollision")
      (Variables|Data|SetbCollected true))
    (:then_1
      (Class|BPICollectable|IsCollected(Message) (Game|GetGameMode) self))
    (:then_2
      (return false))))

(fn RegisterNewCollectable
  (params (CollectableRef :type Actor%20Object%20Reference))
  (return false))